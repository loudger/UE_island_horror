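; Keypad code lock that opens a linked BP_doorNOTkey when the correct code is entered.
; A Box overlap toggles input and a center-dot HUD widget while the lock is unopened.
; Left click matches the player's HitComponent to a button: digits scroll through a rolling display, Reset or a wrong Enter restores the default code.
; A correct Enter swaps in the open screen material, sets IsOpen and clears the door's OpenByCode flag.
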(event `self.ReceiveBeginPlay`
  ;[1 1 1] Обнуляем значение CodeLock вначале игры
  (`TextRenderComponent.K2_SetText` (`self.CodeText`) (`KismetTextLibrary.Conv_StringToText` (`self.DefaultEmptyCode`))))

(event `Key|LeftMouseButton`
  (params (Key :type "Key Structure"))
  (:`Pressed`
    (bind _asbp_first_person_character (cast `/Game/FirstPerson/Blueprints/BP_FirstPersonCharacter` (`GameplayStatics.GetPlayerCharacter` 0)))
    (bind _hit_component (`/Game/FirstPerson/Blueprints/BP_FirstPersonCharacter.Hit Component` _asbp_first_person_character))
    ;[1 1 1] Проверка, что мы смотрим на CodeLock
    (if (`KismetSystemLibrary.IsValid` _hit_component)
      (cast `/Game/Control_Panel/BP_CodeLock` (`ActorComponent.GetOwner` _hit_component))
      ;[1 1 1] Проверяем какая кнопка была нажата
      (for (_array_element _array_index) (`|MakeArray` (`self.button_0`) (`self.button_1`) (`self.button_2`) (`self.button_3`) (`self.button_4`) (`self.button_5`) (`self.button_6`) (`self.button_7`) (`self.button_8`) (`self.button_9`) (`self.button_Reset`) (`self.button_Enter`))
        (set `self.ButtonIndex` _array_index)
        (if (== _array_element _hit_component)
          (`|ExecutionSequence`
            (:`then_0`
              (if (<= (`self.ButtonIndex`) 9)
                ;[1 1 1] Нажата цифра. Обновляем InteredCode + отрисовываем его
                (`self.TextScreenLogic`)
                (`TextRenderComponent.K2_SetText` (`self.CodeText`) (`KismetTextLibrary.Conv_StringToText` (`self.InteredCode`)))))
            (:`then_1`
              (if (== (`self.ButtonIndex`) 10)
                ;[1 1 1] Reset. Обнуление значения
                (bind _output_get (set `self.InteredCode` (`self.DefaultEmptyCode`) :!label _label))
                (`TextRenderComponent.K2_SetText` (`self.CodeText`) (`KismetTextLibrary.Conv_StringToText` _output_get))))
            (:`then_2`
              (if (== (`self.ButtonIndex`) 11)
                ;[1 1 1] Если нажата кнопка Enter. Происходит сравнение кодов
                (if (`KismetStringLibrary.EqualEqual_StrStr` (`self.InteredCode`) (`self.AccessCode`))
                  ;[1 1 1] Устанавливаем значение IsOpen и вызуализируем это
                  (`self.ShowOpenTexture`)
                  (set `self.bIsOpen` true)
                  (bind _asbp_door_notkey (cast `/Game/Blueprint/BP_doorNOTkey` (`self.OpenableActor`)))
                  (`/Game/Blueprint/BP_doorNOTkey.open door` _asbp_door_notkey)
                  (set `/Game/Blueprint/BP_doorNOTkey.openByCode` false _asbp_door_notkey)
                  (else
                    (goto _label)))))))))))

(event `InputAction|Action`
  (params (Key :type "Key Structure")))

(event `self.Box.OnComponentBeginOverlap`
  (params (OverlappedComponent :type "PrimitiveComponent Object Reference") (OtherActor :type "Actor Object Reference") (OtherComp :type "PrimitiveComponent Object Reference") (OtherBodyIndex :type Integer) (bFromSweep :type Boolean) (SweepResult :type "HitResult Structure (by ref)"))
  (bind _returnvalue (`GameplayStatics.GetPlayerController` 0))
  ;[1 1 1] Не даём больше работать с CodeLock, если он уже активирован
  (if (not (`self.bIsOpen`))
    ;[1 1 1] Включаем и выключаем взаимодействие с CodeLock
    (cast `/Game/FirstPerson/Blueprints/BP_FirstPersonCharacter` OtherActor)
    (`self.EnableInput` _returnvalue)
    ;[1 1 1] Включаем и выключаем HUD, чтобы было видно точку по центру экрана
    (bind _returnvalue_2 (`|CreateWidget` "/Game/Control_Panel/HUD_PointAtCenter.HUD_PointAtCenter_C" _returnvalue))
    (`UserWidget.AddToViewport` _returnvalue_2 0)))

(event `self.Box.OnComponentEndOverlap`
  (params (OverlappedComponent :type "PrimitiveComponent Object Reference") (OtherActor :type "Actor Object Reference") (OtherComp :type "PrimitiveComponent Object Reference") (OtherBodyIndex :type Integer))
  ;[1 1 1] Включаем и выключаем взаимодействие с CodeLock
  (cast `/Game/FirstPerson/Blueprints/BP_FirstPersonCharacter` OtherActor)
  (`self.DisableInput` (`GameplayStatics.GetPlayerController` 0))
  ;[1 1 1] Включаем и выключаем HUD, чтобы было видно точку по центру экрана
  (if (`KismetSystemLibrary.IsValid` (stale `self.Box.OnComponentBeginOverlap` _returnvalue_2))
    (`Widget.RemoveFromParent` (stale `self.Box.OnComponentBeginOverlap` _returnvalue_2))))

(fn `ShowOpenTexture`
  ;[1 1 1] Убрать текст кода и показать текстуру Open
  (`SceneComponent.SetVisibility` (`self.CodeText`) false false)
  (`PrimitiveComponent.SetMaterial` (`self.LockPanel`) 1 "/Game/Control_Panel/Materials/HE_ControlScreenOpen.HE_ControlScreenOpen"))

(fn `TextScreenLogic`
  (set `self.InteredCode` (`KismetStringLibrary.Concat_StrStr` (`KismetStringLibrary.Right` (`self.InteredCode`) 3) (`KismetStringLibrary.Conv_IntToString` (`self.ButtonIndex`))))
  (return))

(fn `UserConstructionScript`)