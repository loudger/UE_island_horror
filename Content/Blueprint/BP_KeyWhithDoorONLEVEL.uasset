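; A locked door actor that requires the player's DoorKey1 and sends them to the under_Middle level when used.
; Box overlap enables input and shows one of two text prompts depending on whether the character has the key.
; The Action input drives a timeline that swings the door open or reverses it, guarded by the Time and DoorOpen flags.
; OpenLevelByName fires from the timeline's Update, so travel is requested as the swing starts rather than on Finished.
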(event `self.Box.OnComponentBeginOverlap`
  (params (OverlappedComponent :type "PrimitiveComponent Object Reference") (OtherActor :type "Actor Object Reference") (OtherComp :type "PrimitiveComponent Object Reference") (OtherBodyIndex :type Integer) (bFromSweep :type Boolean) (SweepResult :type "HitResult Structure (by ref)"))
  (`self.EnableInput` (`GameplayStatics.GetPlayerController` 0))
  (bind _asbp_first_person_character (cast `/Game/FirstPerson/Blueprints/BP_FirstPersonCharacter` (`GameplayStatics.GetPlayerCharacter` 0)))
  (if (`/Game/FirstPerson/Blueprints/BP_FirstPersonCharacter.DoorKey1` _asbp_first_person_character)
    (`SceneComponent.SetVisibility` (`self.TextRender2`) true false)
    (else
      (`SceneComponent.SetVisibility` (`self.TextRender1`) true false))))

(event `self.Box.OnComponentEndOverlap`
  (params (OverlappedComponent :type "PrimitiveComponent Object Reference") (OtherActor :type "Actor Object Reference") (OtherComp :type "PrimitiveComponent Object Reference") (OtherBodyIndex :type Integer))
  (`self.DisableInput` (`GameplayStatics.GetPlayerController` 0))
  (`SceneComponent.SetVisibility` (`self.TextRender1`) false false)
  (`SceneComponent.SetVisibility` (`self.TextRender2`) false false))

(event `InputAction|Action`
  (params (Key :type "Key Structure"))
  (:`Pressed`
    (bind _asbp_first_person_character (cast `/Game/FirstPerson/Blueprints/BP_FirstPersonCharacter` (`GameplayStatics.GetPlayerCharacter` 0)))
    (if (`/Game/FirstPerson/Blueprints/BP_FirstPersonCharacter.DoorKey1` _asbp_first_person_character)
      (if (`self.Time`)
        (if (`self.doorOpen?`)
          (set `self.Time` false)
          (bind (_direction _newtrack_0) (`Timeline|TimelineOpenDoor` :!label _label)
            (:`Update`
              (`SceneComponent.K2_SetRelativeRotation` (`self.door`) (`KismetMathLibrary.MakeRotator` 0.0 0.0 (* _newtrack_0 110.0)) false false)
              (set `self.doorOpen?` (not (> _newtrack_0 0.0)))
              (`SceneComponent.SetVisibility` (`self.TextRender1`) false false)
              (`SceneComponent.SetVisibility` (`self.TextRender2`) false false)
              (`GameplayStatics.OpenLevel` "under_Middle"))
            (:`Finished`
              (set `self.Time` true)))
          (else
            (set `self.Time` false)
            (goto _label :!via `ReverseFromEnd`)))))))

(fn `UserConstructionScript`)