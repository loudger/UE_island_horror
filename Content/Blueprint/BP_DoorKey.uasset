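; BP_DoorKey is a pickup key that shows a text prompt facing the player.
; Entering its Box enables input and starts a looping timer that shows the TextRender and rotates it toward the player.
; Leaving disables input and hides the text, but the timer is never cleared.
; Pressing Action sets DoorKey1 on BP_FirstPersonCharacter and destroys the key.
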(event `self.Box.OnComponentBeginOverlap`
  (params (OverlappedComponent :type "PrimitiveComponent Object Reference") (OtherActor :type "Actor Object Reference") (OtherComp :type "PrimitiveComponent Object Reference") (OtherBodyIndex :type Integer) (bFromSweep :type Boolean) (SweepResult :type "HitResult Structure (by ref)"))
  (`self.EnableInput` (`GameplayStatics.GetPlayerController` 0))
  (`KismetSystemLibrary.K2_SetTimerDelegate` (delegate `UpdateTextRender`) 0.01 true))

(event `UpdateTextRender`
  (`self.UpdateText`))

(event `self.Box.OnComponentEndOverlap`
  (params (OverlappedComponent :type "PrimitiveComponent Object Reference") (OtherActor :type "Actor Object Reference") (OtherComp :type "PrimitiveComponent Object Reference") (OtherBodyIndex :type Integer))
  (`self.DisableInput` (`GameplayStatics.GetPlayerController` 0))
  (`SceneComponent.SetVisibility` (`self.TextRender`) false false))

(event `InputAction|Action`
  (params (Key :type "Key Structure"))
  (:`Pressed`
    (bind _asbp_first_person_character (cast `/Game/FirstPerson/Blueprints/BP_FirstPersonCharacter` (`GameplayStatics.GetPlayerCharacter` 0)))
    (set `/Game/FirstPerson/Blueprints/BP_FirstPersonCharacter.DoorKey1` true _asbp_first_person_character)
    (`self.K2_DestroyActor`)))

(fn `UpdateText`
  (bind (_returnvalue_roll _returnvalue_pitch _returnvalue_yaw) (`KismetMathLibrary.BreakRotator` (`KismetMathLibrary.FindLookAtRotation` (`self.K2_GetActorLocation`) (`self.K2_GetActorLocation` (`GameplayStatics.GetPlayerCharacter` 0)))))
  (`SceneComponent.SetVisibility` (`self.TextRender`) true false)
  (`SceneComponent.K2_SetRelativeRotation` (`self.TextRender`) (`KismetMathLibrary.MakeRotator` (- _returnvalue_roll (`self.Return Value X (Roll)`)) (- _returnvalue_pitch (`self.Return Value Y (Pitch)`)) (- _returnvalue_yaw (`self.Return Value Z (Yaw)`))) false false))

(fn `UserConstructionScript`)