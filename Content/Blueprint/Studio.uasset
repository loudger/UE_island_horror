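; Studio is an actor that runs an item inspection session for the player.
; Inspect copies the given mesh onto its Item component, adds an Inspection widget to the viewport, and moves input from the player to itself.
; Pressing the Action input returns control to the player, removes the widget and destroys the Studio, so each instance serves a single inspection.
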(event `/Game/Blueprint/interface/inspect_interface.inspect`
  (params (Player :type "/Game/FirstPerson/Blueprints/BP_FirstPersonCharacter Object Reference") (`Item to focus` :type "StaticMesh Object Reference") (`Item name` :type Text) (`Item description` :type Text))
  (set `self.Player` Player)
  (`StaticMeshComponent.SetStaticMesh` (`self.Item`) `Item to focus`)
  (bind _returnvalue (`|CreateWidget` "/Game/Blueprint/widget/Inspection.Inspection_C"))
  (bind _output_get (set `self.Inspection` _returnvalue))
  (`UserWidget.AddToViewport` _output_get 0)
  (`self.DisableInput` (`self.Player`) (`GameplayStatics.GetPlayerController` 0))
  (`self.EnableInput` null))

(event `InputAction|Action`
  (params (Key :type "Key Structure"))
  (bind _returnvalue (`GameplayStatics.GetPlayerController` 0))
  (:`Pressed`
    (`self.DisableInput` _returnvalue)
    (`self.EnableInput` (`self.Player`) _returnvalue)
    (`Widget.RemoveFromParent` (`self.Inspection`))
    (set `self.Inspection` null)
    (`self.K2_DestroyActor`)))

(fn `UserConstructionScript`)