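; Keyless door Blueprint that the player toggles open and closed with the Action input while overlapping its Box.
; Box overlap enables and disables input, and the press calls Open only when OpenByCode is false.
; A timeline yaws the Door up to 110 degrees, playing forward or reversing from the end based on DoorOpen, which is true at zero track value.
; The Time flag blocks retriggering until the timeline finishes.
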(event `self.Box.OnComponentBeginOverlap`
  (params (OverlappedComponent :type "PrimitiveComponent Object Reference") (OtherActor :type "Actor Object Reference") (OtherComp :type "PrimitiveComponent Object Reference") (OtherBodyIndex :type Integer) (bFromSweep :type Boolean) (SweepResult :type "HitResult Structure (by ref)"))
  (`self.EnableInput` (`GameplayStatics.GetPlayerController` 0)))

(event `self.Box.OnComponentEndOverlap`
  (params (OverlappedComponent :type "PrimitiveComponent Object Reference") (OtherActor :type "Actor Object Reference") (OtherComp :type "PrimitiveComponent Object Reference") (OtherBodyIndex :type Integer))
  (`self.DisableInput` (`GameplayStatics.GetPlayerController` 0)))

(event `InputAction|Action`
  (params (Key :type "Key Structure"))
  (:`Pressed`
    (if (not (`self.openByCode`))
      (`self.open`))))

(event `open door`
  (if (`self.Time`)
    (if (`self.doorOpen?`)
      (set `self.Time` false)
      (bind (_direction _newtrack_0) (`Timeline|TimelineOpenDoor` :!label _label)
        (:`Update`
          (`SceneComponent.K2_SetRelativeRotation` (`self.door`) (`KismetMathLibrary.MakeRotator` 0.0 0.0 (* _newtrack_0 110.0)) false false)
          (set `self.doorOpen?` (not (> _newtrack_0 0.0))))
        (:`Finished`
          (set `self.Time` true)))
      (else
        (set `self.Time` false)
        (goto _label :!via `ReverseFromEnd`)))))

(fn `open`
  (`self.open door`))

(fn `UserConstructionScript`)